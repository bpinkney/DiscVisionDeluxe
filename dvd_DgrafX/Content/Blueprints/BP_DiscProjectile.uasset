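; Disc golf projectile whose velocity and rotation are set by the C++ disc throw simulation (DfisX) until KillControl hands it to PhysX.
; Tick sends batched hits, velocity deltas, logs and lowest-rim ground height to the owning throw actor, repurposing physical material density and damage threshold as grass properties.
; It also steers the spring-arm camera, depenetrates from landscape, and sets mesh, mass and texture per disc type or image file.
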(event MouseInput|EventActorOnClicked
  (params (ButtonPressed :type Key%20Structure))
  ;[1 1 1] Disc Click Detection
  (Development|PrintString "Disky Clickedness")
  (bind _asbp_disc_throw (Utilities|Casting|CastToBP_DiscThrow (Components|GetOwner)))
  (Default|DiscClicked _asbp_disc_throw))

(event EventKillControlwithDelay
  ;[1 1 1] Kill Control
  ; Ends DfisX control of disc and have physx assume all control
  (Utilities|FlowControl|Delay 0.1)
  (Physics|SetEnableGravity (Variables|Default|Getroot) true)
  (if (Variables|Default|Getis_dfisx_simulating)
    (Variables|Default|Setis_dfisx_simulating false)))

(event EventSetDitherLocation
  ;[1 1 1] MATERIAL STUFF
  ; Used to define a see through location for followflight material and eventually foliage dithering
  (Rendering|Material|SetVectorParameterValue "/Game/Materials/FF_dither_effect.FF_dither_effect" "Position_and_size" (Math|Conversions|ToLinearColor(Vector) (Transformation|GetWorldLocation (Variables|Default|Getroot))) :!class /Script/Engine.KismetMaterialLibrary))

(event EventSetDiscMeshandMass
  (params (disc_static_mesh :type enum_disc_form%20Enum :default "PUTTER") (mass_in_kg :type Float%20%28single-precision%29))
  (bind _root (Variables|Default|Getroot))
  ;[1 1 1] Sets the mesh and default texture.
  ; Will override texture if one is found for the mold afterwards in c++
  (Variables|Default|SetMass_in_Kg mass_in_kg)
  (Rendering|Material|SetMaterial _root 0 (Variables|Default|Getdisc_material_instance))
  (switch Utilities|FlowControl|Switch|Switchonenum_disc_form disc_static_mesh
    (:PUTTER
      (Components|StaticMesh|SetStaticMesh (Variables|Default|Getroot) "/Game/DiscStuff/Putter_mesh.Putter_mesh")
      (Rendering|Material|SetTextureParameterValue (Variables|Default|Getdisc_material_instance) "texture_param" "/Game/DiscStuff/Textures/yin_yang.yin_yang"))
    (:MIDRANGE
      (Components|StaticMesh|SetStaticMesh (Variables|Default|Getroot) "/Game/DiscStuff/Midrange_mesh.Midrange_mesh")
      (Rendering|Material|SetTextureParameterValue (Variables|Default|Getdisc_material_instance) "texture_param" "/Game/DiscStuff/Textures/dvd_texture.dvd_texture"))
    (:FAIRWAY
      (Components|StaticMesh|SetStaticMesh _root "/Game/DiscStuff/Fairway_Mesh.Fairway_Mesh")
      (Rendering|Material|SetTextureParameterValue (Variables|Default|Getdisc_material_instance) "texture_param" "/Game/DiscStuff/Textures/stand_here_outline_texture.stand_here_outline_texture"))
    (:DRIVER
      (Components|StaticMesh|SetStaticMesh (Variables|Default|Getroot) "/Game/DiscStuff/Driver_mesh.Driver_mesh")
      (Rendering|Material|SetTextureParameterValue (Variables|Default|Getdisc_material_instance) "texture_param" "/Game/DiscStuff/Textures/huk_lab_texture.huk_lab_texture"))
    (:FRISBEE
      (Components|StaticMesh|SetStaticMesh (Variables|Default|Getroot) "/Game/DiscStuff/frisbee2.frisbee2")
      (Rendering|Material|SetTextureParameterValue (Variables|Default|Getdisc_material_instance) "texture_param" "/Game/DiscStuff/Textures/dvd_texture.dvd_texture")))
  (Class|PrimitiveComponent|SetMassOverrideinKg (Variables|Default|Getroot) "None" (Variables|Default|GetMass_in_Kg) true))

(event EventEndOfThrowCamera
  (Variables|Default|Setis_zooming_out true))

(event EventTick
  (params (DeltaSeconds :type Float%20%28single-precision%29))
  (bind _root (Variables|Default|Getroot))
  (bind _returnvalue (Class|PrimitiveComponent|GetPhysicsAngularVelocityinRadians _root "None"))
  (Utilities|NewMacro0
    (:OutputPin
      ;[1 1 1] End of flight camera panzoom
      ; snapshots current camera angle for post flight zoompan
      (Variables|Default|Setwas_vel_set false)
      (if (Variables|Default|Getis_zooming_out)
        (|postflightzoomandpan))
      ;[1 1 1] Gather all states and state deltas
      (bind _output_get (Variables|Default|Setang_vel_delta (- (Math|Transform|InverseTransformDirection (Transformation|GetActorTransform) (Class|PrimitiveComponent|GetPhysicsAngularVelocityinRadians (Variables|Default|Getroot) "None")) (Variables|Default|Getrecorded_ang_vel))))
      (Variables|Default|Setrecorded_ang_vel (Math|Transform|InverseTransformDirection (Transformation|GetActorTransform) (Class|PrimitiveComponent|GetPhysicsAngularVelocityinRadians (Variables|Default|Getroot) "None")))
      (bind _output_get_2 (Variables|Default|Setlin_vel_delta (- (Transformation|GetVelocity) (Variables|Default|Getrecorded_lin_vel))))
      (bind _output_get_3 (Variables|Default|Setrecorded_lin_vel (Transformation|GetVelocity)))
      (bind _output_get_4 (Variables|Default|Setworld_ang_vel_delta (- (Class|PrimitiveComponent|GetPhysicsAngularVelocityinRadians (Variables|Default|Getroot) "None") (Variables|Default|Getrecorded_world_ang_vel))))
      (Variables|Default|Setrecorded_world_ang_vel _returnvalue)
      ;[1 1 1] Saves shit to flight logs
      (bind _asbp_disc_throw (Utilities|Casting|CastToBP_DiscThrow (Components|GetOwner)))
      (Class|DiscThrow|LogString _asbp_disc_throw (Utilities|String|Append " 
Bueprint States on tick function at :" (Utilities|String|ToString(Float) DeltaSeconds) "  delta seconds"))
      (CallFunction|LogVector (Variables|Default|Getrecorded_lin_vel) "Lin vel: ")
      (CallFunction|LogVector (Variables|Default|Getlin_vel_delta) "Lin vel delta : ")
      (CallFunction|LogVector (Variables|Default|Getrecorded_ang_vel) "Ang vel: ")
      (CallFunction|LogVector (Variables|Default|Getang_vel_delta) "Ang Vel Delta")
      (CallFunction|LogVector (Variables|Default|Getrecorded_world_ang_vel) "World Ang vel: ")
      (CallFunction|LogVector (Variables|Default|Getworld_ang_vel_delta) "World Ang Vel Delta")
      (CallFunction|LogVector (Math|Rotator|GetRotationXVector (Transformation|GetWorldRotation (Variables|Default|Getroot))) "World Ang position")
      ;[1 1 1] just close your eyes and pretend this doesnt exit
      ; TODO: clean up once collision stuff is finalized
      (if (Variables|Default|Getcollision_recorded)
        (Variables|Default|Setcollision_recorded false)
        (bind _asbp_disc_throw_2 (Utilities|Casting|CastToBP_DiscThrow (Components|GetOwner)))
        (Class|DiscThrow|OnCollision _asbp_disc_throw_2 (Transformation|GetActorLocation) (Math|Vector|GetUpVector (Transformation|GetActorRotation)) (Variables|Default|Gethit_locations) (Variables|Default|Gethit_normals) (Variables|Default|Gethit_normal_impulses) _output_get_3 _output_get_2 (Math|Transform|InverseTransformDirection (Transformation|GetActorTransform) (Class|PrimitiveComponent|GetPhysicsAngularVelocityinRadians (Variables|Default|Getroot) "None")) _returnvalue _output_get_4 _output_get (Variables|Default|Gethit_events) DeltaSeconds (Variables|Default|Gethit_frictions) (Variables|Default|Gethit_restitutions))
        (Variables|Default|Sethit_events 0)
        (Utilities|Array|Clear (Variables|Default|Gethit_locations))
        (Utilities|Array|Clear (Variables|Default|Gethit_normals))
        (Utilities|Array|Clear (Variables|Default|Gethit_normal_impulses))))))

(event Collision|EventHit
  (params (MyComp :type Primitive%20Component%20Object%20Reference) (Other :type Actor%20Object%20Reference) (OtherComp :type Primitive%20Component%20Object%20Reference) (bSelfMoved :type Boolean) (HitLocation :type Vector :default "0, 0, 0") (HitNormal :type Vector :default "0, 0, 0") (NormalImpulse :type Vector :default "0, 0, 0") (Hit :type Hit%20Result%20Structure%20%28by%20ref%29))
  ;[1 1 1] Hit Event
  ; note canhappen multiple times per tick but is only run at end of async physics
  ; so result are gathered here and put into an array for consumption
  (bind _output_get (Variables|Default|Sethithithit Hit))
  (Variables|Default|Setcollision_recorded true)
  (Math|Integer|IncrementInt (Variables|Default|Gethit_events)
    (:%20%20
      (Utilities|Array|Add (Variables|Default|Gethit_locations) (- HitLocation (Transformation|GetWorldLocation MyComp)))
      (Utilities|Array|Add (Variables|Default|Gethit_normals) HitNormal)
      (Utilities|Array|Add (Variables|Default|Gethit_normal_impulses) NormalImpulse)
      (Utilities|Array|Add (Variables|Default|Gethit_frictions) (Variables|/Script/Engine.PhysicalMaterial|GetFriction (.PhysMat (Collision|BreakHitResult _output_get))))
      (Utilities|Array|Add (Variables|Default|Gethit_restitutions) (Variables|/Script/Engine.PhysicalMaterial|GetRestitution (.PhysMat (Collision|BreakHitResult _output_get))))
      (bind _asbp_disc_throw (Utilities|Casting|CastToBP_DiscThrow (Components|GetOwner)))
      (Class|DiscThrow|LogHit _asbp_disc_throw true))))

(event EventEndPlay
  (params (EndPlayReason :type EEndPlayReason%20Enum :default "Destroyed"))
  (bind _asbp_disc_throw (Utilities|Casting|CastToBP_DiscThrow (Components|GetOwner)))
  (Class|DiscThrow|EndThrowSimulation _asbp_disc_throw))

(event EventKillControl
  ;[1 1 1] Kill Control
  ; Ends DfisX control of disc and have physx assume all control
  (Physics|SetEnableGravity (Variables|Default|Getroot) true)
  (if (Variables|Default|Getis_dfisx_simulating)
    (Variables|Default|Setis_dfisx_simulating false)))

(event EventSetDiscVelRot
  (params (velocity :type Vector :default "0, 0, 0") (ang_velocity :type Vector :default "0, 0, 0") (ang_position :type Rotator :default "0, 0, 0") (disc_spin_position :type Float%20%28single-precision%29))
  (bind _returnvalue (|Rotatortotarget))
  (bind _returnvalue_2 (|velocityrotator velocity))
  (bind _root (Variables|Default|Getroot))
  (bind _root_2 (Variables|Default|Getroot))
  (bind _root_3 (Variables|Default|Getroot))
  (bind _returnvalue_3 (Transformation|GetWorldLocation _root_3))
  (bind _returnvalue_4 (Transformation|GetWorldLocation _root_2))
  ;[1 1 1] Set disc rotations and velocities
  ; called once per tick by c++ disc throw
  (Physics|SetPhysicsLinearVelocity (Variables|Default|Getroot) velocity false "None")
  (Class|PrimitiveComponent|SetPhysicsAngularVelocityinRadians (Variables|Default|Getroot) ang_velocity false "None")
  (Transformation|SetWorldRotation (Variables|Default|Getroot) (Math|Rotator|CombineRotators ang_position "0, 0, 0") false false)
  (Transformation|AddActorLocalRotation (Math|Rotator|MakeRotator 0.0 0.0 (Math|Float|%(Float) (Math|Trig|RadiansToDegrees disc_spin_position) 3.6e+02)) false false)
  ;[1 1 1] Camera blending
  ; post flight camera done in bp tick
  (if (Variables|Default|Getis_zooming_out)
    _
    (else
      (Transformation|SetWorldRotation (Variables|Default|GetSpringArm) (Math|Rotator|Lerp(Rotator) _returnvalue _returnvalue_2 (|delta0-90=0-1 _returnvalue_2 _returnvalue)) false false)))
  ;[1 1 1] Error detection
  ; TODO remove for build performance
  ; error was never encountered
  ; just for troubleshooting
  (if (Variables|Default|Getwas_vel_set)
    (Development|PrintString "DOUBLE VEL SET WARNING!!" true true "(R=1.000000,G=0.000000,B=0.000000,A=1.000000)" 3e+02)
    (else
      (Variables|Default|Setwas_vel_set true)))
  ;[1 1 1] Depenetration for set rotation
  ; TODO move to c++
  (bind (_outactors _returnvalue_5) (Collision|ComponentOverlapActors _root (Transformation|GetWorldTransform _root) (Utilities|Array|MakeArray "ObjectTypeQuery1") "/Script/Landscape.Landscape"))
  (if _returnvalue_5
    (bind (_outhit _returnvalue_6) (Collision|LineTraceByChannel (+ _returnvalue_3 "0, 0,10.000000") (- _returnvalue_3 "0, 0,10.000000") "TraceTypeQuery1" true (Utilities|Array|MakeArray 0) "ForOneFrame" true "(R=1.000000,G=0.000000,B=0.000000,A=1.000000)" "(R=0.000000,G=1.000000,B=0.000000,A=1.000000)" 6e+01))
    (if _returnvalue_6
      (bind _output_get (Variables|Default|Setlandscape_normal (.normal _outhit)))
      (bind _output_get_2 (Variables|Default|Setheld_location _returnvalue_4))
      (Transformation|SetWorldLocation _root_2 (+ (* _output_get 10) _returnvalue_4) false true)
      (Transformation|SetWorldLocation (Variables|Default|Getroot) _output_get_2 true false))))

(event EventSetDiscTexture
  (params (path_to_texture_file :type String))
  ;[1 1 1] Sets the texture from a called filepath
  ; Used from c++ for both default mold texture and chosen texture
  ;
  ; default texture will be set and then manual texture will override if set
  ; User Defined Texture > Mold Name Texture > Driver/Mid/Putter Texture
  (bind _returnvalue (Class|KismetRenderingLibrary|ImportFileasTexture2D path_to_texture_file))
  (Variables|Default|Setdisc_texture _returnvalue)
  (Rendering|Material|SetTextureParameterValue (Variables|Default|Getdisc_material_instance) "texture_param" _returnvalue)
  (Development|PrintString (Utilities|String|Append "tried to set set texture to " path_to_texture_file) true true "(R=1.000000,G=0.000000,B=0.029831,A=1.000000)" 1e+01))

(event EventBeginPlay
  ;[1 1 1] TODO
  ; gather teepad held target location for camera target
  (Variables|Default|Setcamera_target_position "20000.000000,2000.000000,3000.000000")
  (bind _returnvalue (Rendering|Material|CreateDynamicMaterialInstance "/Game/DiscStuff/Materials/Material_Disc.Material_Disc" "None" :!class /Script/Engine.KismetMaterialLibrary))
  (Variables|Default|Setdisc_material_instance _returnvalue))

(fn ConstructionScript
  (Variables|Default|Setis_dfisx_simulating true))

(fn LogVector
  (params (A :type Vector) (A1 :type String))
  (bind _asbp_disc_throw (Utilities|Casting|CastToBP_DiscThrow (Components|GetOwner))
    (:then
      (Class|DiscThrow|LogString _asbp_disc_throw (Utilities|String|Append A1 (Utilities|String|ToString(Vector) A))))
    (:CastFailed
      _))
  (return))