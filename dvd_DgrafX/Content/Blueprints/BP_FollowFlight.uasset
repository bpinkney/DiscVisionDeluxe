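; Follow-flight trail actor that draws a clickable procedural mesh along the path of its owning disc projectile.
; Each LogPosition call appends vertices offset by movement direction and owner up vector per display shape, then rebuilds the double-sided section with collision.
; Vertex colours use a set hue, alternating with a cycling hue in rainbow mode.
; Unselect applies a translucent ghost material; clicks notify BP_DiscThrow through the owner chain.
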(event OnClicked(ProceduralMesh)
  (params (TouchedComponent :type Primitive%20Component%20Object%20Reference) (ButtonPressed :type Key%20Structure :default "None"))
  (Development|PrintString "Touch my Trail!")
  (bind _asbp_disc_projectile (Utilities|Casting|CastToBP_DiscProjectile (Components|GetOwner)))
  (bind _asbp_disc_throw (Utilities|Casting|CastToBP_DiscThrow (Components|GetOwner _asbp_disc_projectile)))
  (Default|FfClicked _asbp_disc_throw))

(event EventBeginPlay
  (bind _returnvalue (CallFunction|MakeMaterialInstance 4.0 1.0))
  (Variables|Default|SetM_Normal _returnvalue)
  (bind _returnvalue_2 (CallFunction|MakeMaterialInstance 6.0 0.3))
  (Variables|Default|SetM_Ghost _returnvalue_2))

(event Collision|EventActorBeginOverlap
  (params (OtherActor :type Actor%20Object%20Reference)))

(event EventTick
  (params (DeltaSeconds :type Float%20%28single-precision%29)))

(event EventUnselect
  (Rendering|Material|SetMaterial (Variables|Default|GetProceduralMesh) 0 (Variables|Default|GetM_Ghost)))

(event EventLogPosition
  (bind _returnvalue (Transformation|GetActorTransform))
  (bind _actor_to_followflight (Variables|Default|Getactor_to_followflight))
  (bind _triangle_array (Variables|Default|Gettriangle%20array))
  (bind _vertices_array (Variables|Default|Getvertices_array))
  (bind _triangle_array_2 (Variables|Default|Gettriangle%20array))
  (bind _vertices_array_2 (Variables|Default|Getvertices_array))
  (bind _triangle_array_3 (Variables|Default|Gettriangle%20array))
  (bind _vertices_array_3 (Variables|Default|Getvertices_array))
  (bind _returnvalue_2 (Transformation|GetActorTransform _actor_to_followflight))
  (bind _returnvalue_3 (- (.location _returnvalue_2) (.location _returnvalue)))
  (bind _output_get (Variables|Default|Setvector%20to%20last%20FF%20position (- _returnvalue_3 (Variables|Default|GetPosition%20from%20FF%20start))))
  (Variables|Default|SetPosition%20from%20FF%20start _returnvalue_3)
  (Variables|Default|SetFFsideVector (* (Math|Vector|Normalize (Math|Vector|CrossProduct (Math|Vector|GetUpVector (.rotation (Transformation|GetActorTransform (Variables|Default|Getactor_to_followflight)))) _output_get)) (Variables|Default|GetFF_side_draw_width)))
  (Variables|Default|SetFFupVector (* (Math|Vector|GetUpVector (.rotation (Transformation|GetActorTransform (Variables|Default|Getactor_to_followflight)))) (Variables|Default|GetFF_up_draw_height)))
  (switch Utilities|FlowControl|Switch|Switchonenum_ff_display_shape (Variables|Default|Getff_display_shape)
    (:Ribbon
      (CallFunction|AddVerticetoMesh (+ (.location (Transformation|GetActorTransform (Variables|Default|Getactor_to_followflight))) (Variables|Default|GetFFsideVector)) _triangle_array_2 _vertices_array :!label _label)
      (CallFunction|AddVerticetoMesh (- (.location (Transformation|GetActorTransform (Variables|Default|Getactor_to_followflight))) (Variables|Default|GetFFsideVector)) _triangle_array_2 _vertices_array))
    (:Ribbon_Wide
      (goto _label))
    (:Spiral
      (CallFunction|AddVerticetoMesh (+ (.location (Transformation|GetActorTransform (Variables|Default|Getactor_to_followflight))) (Variables|Default|GetFFsideVector)) (Variables|Default|Gettriangle%20array) (Variables|Default|Getvertices_array))
      (CallFunction|AddVerticetoMesh (- (.location (Transformation|GetActorTransform (Variables|Default|Getactor_to_followflight))) (Variables|Default|GetFFupVector)) (Variables|Default|Gettriangle%20array) (Variables|Default|Getvertices_array))
      (CallFunction|AddVerticetoMesh (- (.location (Transformation|GetActorTransform (Variables|Default|Getactor_to_followflight))) (Variables|Default|GetFFsideVector)) (Variables|Default|Gettriangle%20array) (Variables|Default|Getvertices_array))
      (CallFunction|AddVerticetoMesh (+ (.location (Transformation|GetActorTransform (Variables|Default|Getactor_to_followflight))) (Variables|Default|GetFFupVector)) (Variables|Default|Gettriangle%20array) (Variables|Default|Getvertices_array)))
    (:Bandsaw
      (CallFunction|AddVerticetoMesh (+ (.location (Transformation|GetActorTransform (Variables|Default|Getactor_to_followflight))) (* (Variables|Default|GetFFsideVector) 0.7)) _triangle_array _vertices_array_3)
      (CallFunction|AddVerticetoMesh (- (.location (Transformation|GetActorTransform (Variables|Default|Getactor_to_followflight))) (* (Variables|Default|GetFFsideVector) 0.7)) _triangle_array _vertices_array_3)
      (CallFunction|AddVerticetoMesh (+ (.location (Transformation|GetActorTransform (Variables|Default|Getactor_to_followflight))) (Variables|Default|GetFFsideVector)) _triangle_array_3 _vertices_array_2)
      (CallFunction|AddVerticetoMesh (- (.location (Transformation|GetActorTransform (Variables|Default|Getactor_to_followflight))) (Variables|Default|GetFFsideVector)) _triangle_array_3 _vertices_array_2)))
  (CallFunction|RemaketheMesh))

(event EventInit
  (params (set_hue :type Float%20%28single-precision%29) (set_shape :type enum_ff_display_shape%20Enum :default "Ribbon") (set_rainbow :type Boolean))
  (bind _output_get (Variables|Default|SetSet%20hue%20value set_hue))
  (Variables|Default|SetRainbow%20hue%20value _output_get)
  (Variables|Default|Setff_display_shape set_shape)
  (Variables|Default|Setis_rainbow set_rainbow))

(fn ConstructionScript
  (bind _output_get (Variables|Default|Setactor_to_followflight (Components|GetOwner)))
  (Variables|Default|Setvertices_array (Utilities|Array|MakeArray (Transformation|GetActorLocation _output_get) (Transformation|GetActorLocation _output_get)))
  (Variables|Default|Setcolour_array (Utilities|Array|MakeArray "" ""))
  (Utilities|Array|Clear (Variables|Default|GetUV%20array))
  (Rendering|Material|SetMaterial (Variables|Default|GetProceduralMesh) 0 "/Game/Materials/M_FollowFlight.M_FollowFlight"))

(fn AddVerticetoMesh
  (params (vertice%20to%20update :type Vector) (Triangle%20Array :type Array%20of%20Integers) (Vertice%20Array :type Array%20of%20Vectors))
  (bind _colour_array (Variables|Default|Getcolour_array))
  (bind _output_get (Variables|Default|Setvertice%20to%20update vertice%20to%20update))
  (bind _returnvalue (Utilities|Array|Add Vertice%20Array _output_get))
  (Utilities|Array|Add Triangle%20Array _returnvalue)
  (Utilities|Array|Add Triangle%20Array (- _returnvalue 1))
  (Utilities|Array|Add Triangle%20Array (- _returnvalue 2))
  (Utilities|Array|Add Triangle%20Array (- _returnvalue 2))
  (Utilities|Array|Add Triangle%20Array (- _returnvalue 1))
  (Utilities|Array|Add Triangle%20Array _returnvalue)
  (if (Variables|Default|Getis_rainbow)
    (if (Variables|Default|Getrainbow_alternator)
      (Variables|Default|Setrainbow_alternator false)
      (bind _output_get_2 (Variables|Default|SetRainbow%20hue%20value (Math|Float|%(Float) (+ (Variables|Default|GetRainbow%20hue%20value) 2e+01) 3.6e+02)))
      (bind _returnvalue_2 (CallFunction|MakeLinearColor _output_get_2))
      (Utilities|Array|Add _colour_array _returnvalue_2)
      (else
        (Variables|Default|Setrainbow_alternator true)
        (bind _returnvalue_3 (CallFunction|MakeLinearColor (Math|Float|%(Float) (Variables|Default|GetSet%20hue%20value) 3.6e+02) :!label _label))
        (Utilities|Array|Add _colour_array _returnvalue_3)))
    (else
      (goto _label))))

(fn RemaketheMesh
  (Class|ProceduralMeshComponent|CreateMeshSectionLinearColor (Variables|Default|GetProceduralMesh) 0 (Variables|Default|Getvertices_array) (Variables|Default|Gettriangle%20array) 0 0 0 0 0 (Variables|Default|Getcolour_array) 0 true)
  (Rendering|Material|SetMaterial (Variables|Default|GetProceduralMesh) 0 (Variables|Default|GetM_Normal)))

(fn MakeMaterialInstance
  (params (Hue%201-12 :type Float%20%28single-precision%29) (Alpha%200-1 :type Float%20%28single-precision%29))
  (bind _returnvalue (Rendering|Material|CreateDynamicMaterialInstance "/Game/Materials/M_FollowFlight.M_FollowFlight" "None" :!class /Script/Engine.KismetMaterialLibrary))
  (Rendering|Material|SetScalarParameterValue _returnvalue "Opacity" Alpha%200-1 :!class /Script/Engine.MaterialInstanceDynamic)
  (Rendering|Material|SetVectorParameterValue _returnvalue "Base Color" (Class|KismetMathLibrary|HSVtoRGB (* 30 Hue%201-12) 1.0 1.0 1.0) :!class /Script/Engine.MaterialInstanceDynamic)
  (return _returnvalue))

(fn MakeLinearColor
  (params (Hue%201-12 :type Float%20%28single-precision%29))
  (return (Class|KismetMathLibrary|HSVtoRGB Hue%201-12 1.0 0.2 1.0)))