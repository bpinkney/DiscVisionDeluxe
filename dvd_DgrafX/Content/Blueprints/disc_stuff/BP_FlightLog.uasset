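; BP_FlightLog is a debug recorder for a disc projectile's flight.
; LogPosition stores timestamp, transform, text and hit flag in parallel arrays, while helper functions amend the latest entry's text or hit flag.
; ActivateDisplayedDiscTrail spawns labeled display discs, initially filtered by recent hits, then for every sample on later calls.
; DumpStringLog prints the text entries to the output log, and FlightLogLaunch is an empty stub.
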(event EventBeginPlay)

(event Collision|EventActorBeginOverlap
  (params (OtherActor :type Actor%20Object%20Reference)))

(event EventLogPosition
  (params (DeltaTime :type Float%20%28single-precision%29))
  (bind _output_get (Variables|Default|Setrunning_timestamp (+ DeltaTime (Variables|Default|Getrunning_timestamp))))
  (Utilities|Array|Add (Variables|Default|Gettimestamp_arr) _output_get)
  (Utilities|Array|Add (Variables|Default|Gettransform_arr) (Transformation|GetWorldTransform (Variables|/Script/Engine.Actor|GetRootComponent (Variables|Default|Getptr_disc_projectile))))
  (Utilities|Array|Add (Variables|Default|Gettext_log_arr) (Utilities|String|Append "t-" (Utilities|String|ToString(Float) (Variables|Default|Getrunning_timestamp)) " seconds  
"))
  (Utilities|Array|Add (Variables|Default|Gethit_log_arr) false))

(fn ConstructionScript
  (Variables|Default|Setrunning_timestamp 0.0)
  (Utilities|Array|Clear (Variables|Default|Gettransform_arr))
  (Utilities|Array|Clear (Variables|Default|Gettimestamp_arr))
  (Utilities|Array|Clear (Variables|Default|Gethit_log_arr))
  (Utilities|Array|Clear (Variables|Default|Gettext_log_arr)))

(fn ActivateDisplayedDiscTrail
  (Development|PrintString "Displaying debug discs")
  (for (_array_element _array_index) (Variables|Default|Gettransform_arr)
    (if (Utilities|Array|Get(acopy) (Variables|Default|Gethit_log_arr) _array_index)
      (Variables|Default|Setframes%20without%20hit 0)
      (else
        (Math|Integer|IncrementInt (Variables|Default|Getframes%20without%20hit)
          (:%20%20
            _))))
    (if (Math|Boolean|ORBoolean (Utilities|Array|Get(acopy) (Variables|Default|Gethit_log_arr) _array_index) (< (Variables|Default|Getframes%20without%20hit) 3) (Variables|Default|Gethits_already_displayed))
      (Game|SpawnActorfromClass "/Game/Blueprints/disc_stuff/BP_FlightLogDisplayDisc.BP_FlightLogDisplayDisc_C" _array_element "Undefined" 0 (Utilities|Text|ToText(String) (Utilities|Array|Get(acopy) (Variables|Default|Gettext_log_arr) _array_index)) 0)))
  (Variables|Default|Sethits_already_displayed true))

(fn FlightLogString
  (params (NewParam :type String))
  (bind _text_log_arr (Variables|Default|Gettext_log_arr))
  (bind _returnvalue (Utilities|Array|LastIndex _text_log_arr))
  (Utilities|Array|SetArrayElem _text_log_arr _returnvalue (Utilities|String|Append (Utilities|Array|Get(acopy) _text_log_arr _returnvalue) NewParam " 
")))

(fn DumpStringLog
  (Development|PrintString " 
Dumping string logs to output log...----------------------------------------------. 
")
  (for _array_element (Variables|Default|Gettext_log_arr)
    (Development|PrintString _array_element false))
  (Development|PrintString " 
Dump complete.----------------------------------------------------------------------------- 
"))

(fn FlightLogHit
  (params (issa_hit :type Boolean))
  (bind _hit_log_arr (Variables|Default|Gethit_log_arr))
  (Utilities|Array|SetArrayElem _hit_log_arr (Utilities|Array|LastIndex _hit_log_arr) issa_hit))

(fn FlightLogLaunch
  (params (issa_launch :type Boolean)))