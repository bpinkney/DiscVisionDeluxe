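; BP_DiscThrow is a disc-throw actor that handles projectile cleanup and relays logging to a flight log.
; String and hit events forward to BP_FlightLog by casting PtrFlightLog, and the log dumps on request or after a delay from BeginPlay.
; DestroyDiscs removes all BP_DiscProjectile actors.
; The two click functions print debug text and activate the flight log's displayed disc trail.
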(event EventBeginPlay
  (Utilities|FlowControl|Delay 15.0)
  (bind _asbp_flight_log (Utilities|Casting|CastToBP_FlightLog (Variables|Default|Getptr_flight_log)))
  (Default|DumpStringLog _asbp_flight_log))

(event Collision|EventActorBeginOverlap
  (params (OtherActor :type Actor%20Object%20Reference)))

(event EventTick
  (params (DeltaSeconds :type Float%20%28single-precision%29)))

(event EventDestroyDiscs
  (bind _outactors (Actor|GetAllActorsOfClass "/Game/Blueprints/BP_DiscProjectile.BP_DiscProjectile_C"))
  (Actor|DestroyActor _outactors))

(event EventLogString
  (params (stringlog :type String))
  (bind _asbp_flight_log (Utilities|Casting|CastToBP_FlightLog (Variables|Default|Getptr_flight_log)))
  (Default|FlightLogString _asbp_flight_log stringlog))

(event EventDumpStringLog
  (bind _asbp_flight_log (Utilities|Casting|CastToBP_FlightLog (Variables|Default|Getptr_flight_log)))
  (Default|DumpStringLog _asbp_flight_log))

(event EventLogHit
  (params (issa_hit :type Boolean))
  (Class|DiscThrow|LogString (Utilities|String|Append "hit = " (Utilities|String|ToString(Boolean) issa_hit) " 
"))
  (bind _asbp_flight_log (Utilities|Casting|CastToBP_FlightLog (Variables|Default|Getptr_flight_log))
    (:then
      (Default|FlightLogHit _asbp_flight_log issa_hit))
    (:CastFailed
      (Development|PrintString "cast failed in disc throw for log hit"))))

(fn ConstructionScript)

(fn FfClicked
  (Development|PrintString "ff clicked?")
  (bind _asbp_flight_log (Utilities|Casting|CastToBP_FlightLog (Variables|Default|Getptr_flight_log)))
  (Default|ActivateDisplayedDiscTrail _asbp_flight_log))

(fn DiscClicked
  (Development|PrintString "disc lcicked?")
  (bind _asbp_flight_log (Utilities|Casting|CastToBP_FlightLog (Variables|Default|Getptr_flight_log)))
  (Default|ActivateDisplayedDiscTrail _asbp_flight_log))