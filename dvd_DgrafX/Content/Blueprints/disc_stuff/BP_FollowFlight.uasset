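; Flight trail actor that draws a procedural mesh behind its owning disc in one of ten selectable shapes.
; Each LogPosition call derives side and up vectors from the owner's movement, appends the shape's vertices as double-sided triangles and rebuilds the mesh section.
; Init sets shape, fixed or rainbow vertex colours, and solid and ghost dynamic materials that Select and Unselect swap.
; Clicking the trail calls FfClicked on the BP_DiscThrow owning the projectile.
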(event OnClicked(ProceduralMesh)
  (params (TouchedComponent :type Primitive%20Component%20Object%20Reference) (ButtonPressed :type Key%20Structure))
  (Development|PrintString "Touch my Trail!")
  (bind _asbp_disc_projectile (Utilities|Casting|CastToBP_DiscProjectile (Components|GetOwner)))
  (bind _asbp_disc_throw (Utilities|Casting|CastToBP_DiscThrow (Components|GetOwner _asbp_disc_projectile)))
  (Default|FfClicked _asbp_disc_throw))

(event Collision|EventActorBeginOverlap
  (params (OtherActor :type Actor%20Object%20Reference)))

(event EventTick
  (params (DeltaSeconds :type Float%20%28single-precision%29)))

(event EventUnselect
  (Rendering|Material|SetMaterial (Variables|Default|GetProceduralMesh) 0 (Variables|Default|GetM_Ghost)))

(event EventSelect
  (Rendering|Material|SetMaterial (Variables|Default|GetProceduralMesh) 0 (Variables|Default|GetM_Normal)))

(event EventLogPosition
  (|makevectors(kindaspency))
  (switch Utilities|FlowControl|Switch|Switchonenum_ff_display_shape (Variables|Default|Getff_display_shape)
    (:Ribbon
      (|basicribbon))
    (:Ribbon_Wide
      (|wideribbon))
    (:Art_Diamonds
      (|diamondchain))
    (:Tube
      (|tube))
    (:Wide_Tube
      (|widetube))
    (:Tie_Fighter
      (|tiefighter))
    (:Trapezoid
      (|floatingtrapezoids))
    (:Wrong_Way
      (|wrongway))
    (:Zig_Zag
      (|zigzag))
    (:Bandsaw
      (|Bandsaw)))
  (CallFunction|RemaketheMesh))

(event EventInit
  (params (set_disc_hue :type Float%20%28single-precision%29) (set_player_colour :type Color%20Structure) (set_shape :type enum_ff_display_shape%20Enum :default "Ribbon") (set_rainbow :type Boolean))
  (bind _output_get (Variables|Default|SetSet%20disc%20hue%20value set_disc_hue))
  (Variables|Default|SetRainbow%20hue%20value _output_get)
  (Variables|Default|Setff_display_shape set_shape)
  (Variables|Default|Setis_rainbow set_rainbow)
  (bind _returnvalue (CallFunction|MakeMaterialInstance 4.0 1.0 set_player_colour))
  (Variables|Default|SetM_Normal _returnvalue)
  (bind _returnvalue_2 (CallFunction|MakeMaterialInstance 6.0 0.3 set_player_colour))
  (Variables|Default|SetM_Ghost _returnvalue_2)
  (Transformation|SetWorldLocationAndRotation (Variables|Default|GetDefaultSceneRoot) "0, 0, 0" "0, 0, 0" false false))

(fn ConstructionScript
  (bind _output_get (Variables|Default|Setactor_to_followflight (Components|GetOwner)))
  (Variables|Default|Setvertices_array (Utilities|Array|MakeArray (Transformation|GetActorLocation _output_get) (Transformation|GetActorLocation _output_get)))
  (Variables|Default|SetPrev%20Target%20Location (Transformation|GetActorLocation _output_get))
  (Variables|Default|SetCurrent%20Target%20Location (Transformation|GetActorLocation _output_get))
  (Variables|Default|Setcolour_array (Utilities|Array|MakeArray "" ""))
  (Utilities|Array|Clear (Variables|Default|GetUV%20array))
  (Rendering|Material|SetMaterial (Variables|Default|GetProceduralMesh) 0 "/Game/Materials/M_FollowFlight.M_FollowFlight"))

(fn AddVerticetoMesh
  (params (vertice%20to%20update :type Vector) (Triangle%20Array :type Array%20of%20Integers) (Vertice%20Array :type Array%20of%20Vectors))
  (bind _colour_array (Variables|Default|Getcolour_array))
  (bind _output_get (Variables|Default|Setvertice%20to%20update vertice%20to%20update))
  (bind _returnvalue (Utilities|Array|Add Vertice%20Array _output_get))
  (Utilities|Array|Add Triangle%20Array _returnvalue)
  (Utilities|Array|Add Triangle%20Array (- _returnvalue 1))
  (Utilities|Array|Add Triangle%20Array (- _returnvalue 2))
  (Utilities|Array|Add Triangle%20Array (- _returnvalue 2))
  (Utilities|Array|Add Triangle%20Array (- _returnvalue 1))
  (Utilities|Array|Add Triangle%20Array _returnvalue)
  (if (Variables|Default|Getis_rainbow)
    (bind _output_get_2 (Variables|Default|SetRainbow%20hue%20value (Math|Float|%(Float) (+ (Variables|Default|GetRainbow%20hue%20value) 15.0) 3.6e+02)))
    (bind _returnvalue_2 (CallFunction|MakeLinearColor _output_get_2))
    (Utilities|Array|Add _colour_array _returnvalue_2)
    (else
      (bind _returnvalue_3 (CallFunction|MakeLinearColor (Math|Float|%(Float) (Variables|Default|GetSet%20disc%20hue%20value) 3.6e+02)))
      (Utilities|Array|Add _colour_array _returnvalue_3))))

(fn RemaketheMesh
  (Class|ProceduralMeshComponent|CreateMeshSectionLinearColor (Variables|Default|GetProceduralMesh) 0 (Variables|Default|Getvertices_array) (Variables|Default|Gettriangle%20array) 0 0 0 0 0 (Variables|Default|Getcolour_array) 0 true)
  (Rendering|Material|SetMaterial (Variables|Default|GetProceduralMesh) 0 (Variables|Default|GetM_Normal)))

(fn MakeMaterialInstance
  (params (Disc%20Hue%201-12 :type Float%20%28single-precision%29) (Alpha%200-1 :type Float%20%28single-precision%29) (Player%20Colour :type Color%20Structure))
  (bind _returnvalue (Rendering|Material|CreateDynamicMaterialInstance "/Game/Materials/M_FollowFlight.M_FollowFlight" "None" :!class /Script/Engine.KismetMaterialLibrary))
  (Rendering|Material|SetScalarParameterValue _returnvalue "Opacity" Alpha%200-1 :!class /Script/Engine.MaterialInstanceDynamic)
  (Rendering|Material|SetVectorParameterValue _returnvalue "Base Color" (Class|KismetMathLibrary|HSVtoRGB (* 30 Disc%20Hue%201-12) 1.0 1.0 1.0) :!class /Script/Engine.MaterialInstanceDynamic)
  (Rendering|Material|SetVectorParameterValue _returnvalue "player_colour" (Math|Conversions|ToLinearColor(Color) Player%20Colour) :!class /Script/Engine.MaterialInstanceDynamic)
  (return _returnvalue))

(fn MakeLinearColor
  (params (Hue%201-12 :type Float%20%28single-precision%29))
  (return (Class|KismetMathLibrary|HSVtoRGB Hue%201-12 1.0 0.2 1.0)))

(fn AddVertice
  (params (B :type Vector))
  (CallFunction|AddVerticetoMesh (+ (Transformation|GetActorLocation (Variables|Default|Getactor_to_followflight)) B) (Variables|Default|Gettriangle%20array) (Variables|Default|Getvertices_array)))

(fn RebaseVertArray
  (params (Vert%201 :type Vector%20%28by%20ref%29) (Vert%202 :type Vector%20%28by%20ref%29))
  (bind _vertices_array (Variables|Default|Getvertices_array))
  (bind _colour_array (Variables|Default|Getcolour_array))
  (Utilities|Array|Add _vertices_array Vert%201)
  (Utilities|Array|Add _vertices_array Vert%202)
  (Variables|Default|Setrainbow_alternator true)
  (bind _returnvalue (CallFunction|MakeLinearColor (Math|Float|%(Float) (Variables|Default|GetSet%20disc%20hue%20value) 3.6e+02)))
  (Utilities|Array|Add _colour_array _returnvalue)
  (Utilities|Array|Add _colour_array _returnvalue))

(fn RewindRainbow
  (Variables|Default|SetRainbow%20hue%20value (- (Variables|Default|GetRainbow%20hue%20value) 3e+01)))