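; BP_DiscCharacter is the disc-throwing character that previews a throw pose and launches discs from debug inputs.
; SetThrowPoses maps hyzer and nose angle onto a fake disc, pitch onto a spring arm, and direction onto the Pug component.
; FireFromDebug spawns BP_DiscThrow, offsets position and direction by Pug location and actor yaw, and derives roll and pitch from the fake disc's up vector.
; The mold input is unused.
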(event EventBeginPlay)

(event Collision|EventActorBeginOverlap
  (params (OtherActor :type Actor%20Object%20Reference)))

(event EventTick
  (params (DeltaSeconds :type Float%20%28single-precision%29)))

(fn ConstructionScript)

(fn SetThrowPoses
  (params (hyzer :type Float%20%28single-precision%29) (nose_angle :type Float%20%28single-precision%29) (pitch :type Float%20%28single-precision%29) (direction :type Float%20%28single-precision%29))
  (Transformation|SetRelativeRotation (Variables|Default|Getfakedisc) (Math|Rotator|MakeRotator hyzer (* nose_angle -1.0) 0.0) false false)
  (Transformation|SetRelativeRotation (Variables|Default|GetSpringArm2) (Math|Rotator|MakeRotator 0.0 (* pitch -1.0) -9e+01) false false)
  (Transformation|SetRelativeLocationAndRotation (Variables|Default|GetPug) (Math|Vector|MakeVector 0.0 0.0 -9e+01) (Math|Rotator|MakeRotator 0.0 0.0 (+ direction -9e+01)) false false))

(fn FirefromDebug
  (params (disc_mold_enum :type Integer) (thrown_disc_position :type Vector) (thrown_disc_speed :type Float%20%28single-precision%29) (thrown_disc_direction :type Float%20%28single-precision%29) (thrown_disc_loft :type Float%20%28single-precision%29) (thrown_disc_spin_percent :type Float%20%28single-precision%29) (thrown_disc_wobble :type Float%20%28single-precision%29))
  (bind _fakedisc (Variables|Default|Getfakedisc))
  (bind _returnvalue (Math|Vector|GetUpVector _fakedisc))
  (bind _returnvalue_2 (Math|Conversions|RotationFromXVector _returnvalue))
  (bind _returnvalue_3 (- 9e+01 (.pitch _returnvalue_2)))
  (bind _returnvalue_4 (Game|SpawnActorfromClass "/Game/Blueprints/BP_DiscThrow.BP_DiscThrow_C" (Math|Transform|MakeTransform "0, 0, 0") "AlwaysSpawn" self 0))
  (Class|DiscThrow|NewThrowCameraRelative _returnvalue_4 0 (+ thrown_disc_position (Transformation|GetWorldLocation (Variables|Default|GetPug))) thrown_disc_speed (+ thrown_disc_direction (.yaw (Transformation|GetActorRotation))) thrown_disc_loft (* _returnvalue_3 (Math|Trig|Sin(Degrees) (.yaw _returnvalue_2)) 1.0) (* (Math|Trig|Cos(Degrees) (.yaw _returnvalue_2)) _returnvalue_3 -1.0) thrown_disc_spin_percent thrown_disc_wobble))