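; FollowFlight draws a ribbon trail along the path of a followed actor using a procedural mesh.
; Each external LogPosition call adds two vertices either side of the actor's offset from this actor, along the cross product of its up vector and movement delta.
; AddVerticeToMesh appends double-sided strip triangles, and RemakeTheMesh rebuilds the whole ever-growing section with the M_FollowFlight material.
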(event EventBeginPlay)

(event Collision|EventActorBeginOverlap
  (params (OtherActor :type Actor%20Object%20Reference)))

(event EventTick
  (params (DeltaSeconds :type Float%20%28single-precision%29)))

(fn ConstructionScript
  (bind _output_get (Variables|Default|Setactor_to_followflight (Variables|Default|Getactor_to_followflight)))
  (Variables|Default|Setvertices_array (Utilities|Array|MakeArray (Transformation|GetActorLocation _output_get) (Transformation|GetActorLocation _output_get)))
  (Rendering|Material|SetMaterial (Variables|Default|GetProceduralMesh) 0 "/Game/Materials/M_FollowFlight.M_FollowFlight"))

(fn LogPosition
  (params (Actor :type Actor%20Object%20Reference))
  (bind _output_get (Variables|Default|Setactor_to_followflight Actor))
  (bind _output_get_2 (Variables|Default|Setvector%20to%20last%20FF%20position (- (- (.location (Transformation|GetActorTransform _output_get)) (.location (Transformation|GetActorTransform))) (Variables|Default|GetPosition%20from%20FF%20start))))
  (bind _output_get_3 (Variables|Default|SetPosition%20from%20FF%20start (- (.location (Transformation|GetActorTransform _output_get)) (.location (Transformation|GetActorTransform)))))
  (bind _output_get_4 (Variables|Default|SetFFpoint1 (- _output_get_3 (* (Math|Vector|Normalize (Math|Vector|CrossProduct (Math|Vector|GetUpVector (.rotation (Transformation|GetActorTransform _output_get))) _output_get_2)) 40))))
  (CallFunction|AddVerticetoMesh _output_get_4)
  (bind _output_get_5 (Variables|Default|SetFFpoint2 (+ _output_get_3 (* (Math|Vector|Normalize (Math|Vector|CrossProduct (Math|Vector|GetUpVector (.rotation (Transformation|GetActorTransform _output_get))) _output_get_2)) 40))))
  (CallFunction|AddVerticetoMesh _output_get_5)
  (CallFunction|RemaketheMesh))

(fn AddVerticetoMesh
  (params (vertice%20to%20update :type Vector))
  (bind _triangle_array (Variables|Default|Gettriangle%20array))
  (bind _output_get (Variables|Default|Setvertice%20to%20update vertice%20to%20update))
  (bind _returnvalue (Utilities|Array|Add (Variables|Default|Getvertices_array) _output_get))
  (Utilities|Array|Add _triangle_array _returnvalue)
  (Utilities|Array|Add _triangle_array (- _returnvalue 1))
  (Utilities|Array|Add _triangle_array (- _returnvalue 2))
  (Utilities|Array|Add _triangle_array (- _returnvalue 2))
  (Utilities|Array|Add _triangle_array (- _returnvalue 1))
  (Utilities|Array|Add _triangle_array _returnvalue))

(fn RemaketheMesh
  (Class|ProceduralMeshComponent|CreateMeshSectionLinearColor (Variables|Default|GetProceduralMesh) 0 (Variables|Default|Getvertices_array) (Variables|Default|Gettriangle%20array) 0 0 0 0 0 0 0 false)
  (Rendering|Material|SetMaterial (Variables|Default|GetProceduralMesh) 0 "/Game/Materials/M_FollowFlight.M_FollowFlight"))