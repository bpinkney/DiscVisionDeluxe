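; BP_CameraManager switches a controller's view target between the owning disc character, thrown discs, tee pads and the bag maker in a disc game.
; Disc focus increments a live-disc count and blends to the disc after a delay.
; When the last disc's flight camera finishes, a five-second timer returns the view to the character.
; Tee pad (picked by index) and bag maker focus find set pieces by class and blend near-instantly.
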(event Custom|dummyevent
  (bind _asdisc_character (Utilities|Casting|CastToDiscCharacter (Components|GetOwner)))
  (Game|Player|SetViewTargetwithBlend (Variables|Default|Gettarget_controller) _asdisc_character 0.0 "VTBlend_Cubic" 0.0 false))

(event Custom|Post%20disc%20flight%20camera%20done
  (bind _result (Math|Integer|DecrementInt (Variables|Default|Getlive_disc_count))
    (:%20%20
      (if (== _result 0)
        (Utilities|Time|SetTimerbyEvent (delegate Custom|dummyevent) 5.0)))))

(event EventBeginPlay
  (Variables|Default|Setlive_disc_count 0))

(event Collision|EventActorBeginOverlap
  (params (OtherActor :type Actor%20Object%20Reference)))

(event EventTick
  (params (DeltaSeconds :type Float%20%28single-precision%29)))

(event EventFocusonTeepad
  (params (teepad_id :type Integer))
  (bind _outactors (Actor|GetAllActorsOfClass "/Game/Editor_Set_Pieces/TeePad_setpiece.TeePad_setpiece_C"))
  (Game|Player|SetViewTargetwithBlend (Variables|Default|Gettarget_controller) (Utilities|Array|Get(acopy) _outactors teepad_id) 0.0001 "VTBlend_Cubic" 0.0 false))

(event EventFocusonBagMaker
  (bind _outactors (Actor|GetAllActorsOfClass "/Game/Editor_Set_Pieces/BagMaker_setpiece.BagMaker_setpiece_C"))
  (Game|Player|SetViewTargetwithBlend (Variables|Default|Gettarget_controller) (Utilities|Array|Get(acopy) _outactors) 0.0001 "VTBlend_Cubic" 0.0 false))

(event EventSetPlayerTarget
  (params (player_target :type Player%20Controller%20Object%20Reference))
  (Variables|Default|Settarget_controller player_target))

(event EventFocusonPlayer
  (bind _asdisc_character (Utilities|Casting|CastToDiscCharacter (Components|GetOwner)))
  (Game|Player|SetViewTargetwithBlend (Variables|Default|Gettarget_controller) _asdisc_character 0.0 "VTBlend_Cubic" 0.0 false))

(event EventFocusonDisc
  (params (new_disc_target :type Actor%20Object%20Reference))
  (Math|Integer|IncrementInt (Variables|Default|Getlive_disc_count)
    (:%20%20
      (Utilities|FlowControl|Delay (Variables|Default|Getblend_to_disc_delay))
      (bind _output_get (Variables|Default|Settarget_disc new_disc_target))
      (Game|Player|SetViewTargetwithBlend (Variables|Default|Gettarget_controller) _output_get (Variables|Default|Getblend_to_disc_time) "VTBlend_Cubic" 0.0 false))))

(fn ConstructionScript)