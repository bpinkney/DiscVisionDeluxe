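; Disc golf character Blueprint that records tee pad spawn points and sets the debug HUD minimap target at start.
; BeginPlay stores the spawn transform of every TeePad_setpiece in TeepadLocations.
; The same loop body runs a short Delay, then calls SetMinimapTarget on the first player's debug HUD.
; FireFromDebug declares disc throw parameters but has an empty body, and a slow-motion time dilation node is left unconnected.
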(event EventBeginPlay
  (bind _outactors (Actor|GetAllActorsOfClass "/Game/Editor_Set_Pieces/TeePad_setpiece.TeePad_setpiece_C"))
  (for _array_element _outactors
    (Utilities|Array|Add (Variables|Default|Getteepad_locations) (Transformation|GetWorldTransform (Variables|/Game/Editor_Set_Pieces/TeePad_setpiece.TeePad_setpiece_C|Getspawnpoint _array_element)))
    (Utilities|FlowControl|Delay 0.2)
    (bind _ashud_debug_hud (Utilities|Casting|CastToHUD_Debug_HUD (HUD|GetHUD (Game|GetPlayerController 0))))
    (Class|RangeHUD|SetMinimapTarget _ashud_debug_hud 1)))

(event Collision|EventActorBeginOverlap
  (params (OtherActor :type Actor%20Object%20Reference)))

(event EventTick
  (params (DeltaSeconds :type Float%20%28single-precision%29)))

(fn ConstructionScript)

(fn FirefromDebug
  (params (disc_mold_enum :type Integer) (thrown_disc_position :type Vector) (thrown_disc_speed :type Float%20%28single-precision%29) (thrown_disc_direction :type Float%20%28single-precision%29) (thrown_disc_loft :type Float%20%28single-precision%29) (thrown_disc_spin_percent :type Float%20%28single-precision%29) (thrown_disc_wobble :type Float%20%28single-precision%29)))